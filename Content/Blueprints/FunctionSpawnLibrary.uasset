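; Spawn helper library that maps an item name to its class, covering resources, crystals, food, weapons, lightsabers and a small wooden house.
; Its one function, GetClassWithName, uses a hardcoded switch on the name to set ClassToReturn, with all cases converging on a single return.
; Names must match the case labels, some of which carry a "C" suffix, and no default case is handled.
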(fn GetClasswithName
  (params (Name :type String))
  (switch string Name
    (:Wood_C
      (LocalVariables|SetClassToReturn "/Game/BluePrintAntonin/Items/Wood.Wood_C"))
    (:Stone_C
      (LocalVariables|SetClassToReturn "/Game/BluePrintAntonin/Items/Stone.Stone_C"))
    (:Little_House_Wood
      (LocalVariables|SetClassToReturn "/Game/BluePrintAntonin/Items/Little_House_Wood.Little_House_Wood_C"))
    (:Weapon_Axe
      (LocalVariables|SetClassToReturn "/Game/BluePrintAntonin/Weapon/Weapon_Axe.Weapon_Axe_C"))
    (:Weapon_Sword
      (LocalVariables|SetClassToReturn "/Game/BluePrintAntonin/Weapon/Weapon_Sword.Weapon_Sword_C"))
    (:Apple_C
      (LocalVariables|SetClassToReturn "/Game/BluePrintAntonin/Items/Apple.Apple_C"))
    (:Wood_Planche
      (LocalVariables|SetClassToReturn "/Game/BluePrintAntonin/Items/Wood_Planche.Wood_Planche_C"))
    (:Metal_C
      (LocalVariables|SetClassToReturn "/Game/BluePrintAntonin/Items/Metal.Metal_C"))
    (:LightSaberGreen
      (LocalVariables|SetClassToReturn "/Game/BluePrintAntonin/Weapon/LightSaberGreen.LightSaberGreen_C"))
    (:LightSaberRed
      (LocalVariables|SetClassToReturn "/Game/BluePrintAntonin/Weapon/LightSaberRed.LightSaberRed_C"))
    (:RedCrystal_C
      (LocalVariables|SetClassToReturn "/Game/BluePrintAntonin/Items/RedCrystal.RedCrystal_C"))
    (:GreenCrystal_C
      (LocalVariables|SetClassToReturn "/Game/BluePrintAntonin/Items/GreenCrystal.GreenCrystal_C"))
    (:Weapon_PickAxe
      (LocalVariables|SetClassToReturn "/Game/BluePrintAntonin/Weapon/Weapon_PickAxe.Weapon_PickAxe_C"))
    (:Weapon_Machette
      (LocalVariables|SetClassToReturn "/Game/BluePrintAntonin/Weapon/Weapon_Machette.Weapon_Machette_C")))
  (return (LocalVariables|GetClassToReturn)))