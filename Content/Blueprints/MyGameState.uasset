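; Game state for Reborn Society that holds item and crafting lookup data and handles player persistence.
; BeginPlay builds a hard-coded name-to-class table and two-ingredient recipe list.
; SpawnMyPlayer loads menu and main save slots, then respawns saved inventory and weapon by name to initialize the character.
; Saving is unfinished: event calls are disconnected and the data-filling logic never runs, so SaveGame would write an unfilled object.
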(event EventBeginPlay
  (CallFunction|InitNameClassTable)
  (CallFunction|InitDataCraft))

(event EventEndPlay
  (params (EndPlayReason :type EEndPlayReason%20Enum :default "ActorDestroyed"))
  (switch Utilities|FlowControl|Switch|SwitchonEEndPlayReason EndPlayReason))

(fn ConstructionScript)

(fn SaveGame
  ;[1 1 1] Init Save
  (bind _returnvalue (SaveGame|CreateSaveGameObject "/Game/Blueprints/SavingGame/SaveData.SaveData_C"))
  (bind _assave_data (Utilities|Casting|CastToSaveData _returnvalue))
  (Variables|Saveandload|SetSaveGameInstance _assave_data)
  ;[1 1 1] Fill the data
  (Saveandload|FillDataforSave)
  ;[1 1 1] Sauvegarde
  (SaveGame|SaveGametoSlot (Variables|Saveandload|GetSaveGameInstance) "SauvegardeRebornSociety"))

(fn FillDataforSave)

(fn GetAllPlayers
  (bind _outactors (Actor|GetAllActorsOfClass "/Game/BluePrintAntonin/CharacterAnto.CharacterAnto_C"))
  (return _outactors))

(fn MakeSaveDataStructforPlayer
  (params (Player :type Character%20Anto%20Object%20Reference)))

(fn PlayerAlReadyinSave
  (params (NameToTest :type Name)))

(fn SpawnWeaponWithname
  (params (Weap :type String))
  (CallFunction|GetClasswithName Weap)
  (bind _returnvalue (Game|SpawnActorfromClass (Variables|Default|GetClassFind) (Math|Transform|MakeTransform "1000.000000,1000.000000,1000.000000") false 0))
  (bind _asbase_inventory_actor (Utilities|Casting|CastToBaseInventoryActor _returnvalue))
  (return _asbase_inventory_actor))

(fn GetClassWithname
  (params (Name :type String))
  (for _array_element (Variables|Default|GetNameClassTable)
    (if (Utilities|Enum|Equal(Enum) Name (Utilities|String|ToString(Name) (.Name (Utilities|Struct|BreakNameClassItem _array_element))))
      (Variables|Default|SetClassFind (.Classe (Utilities|Struct|BreakNameClassItem _array_element))))))

(fn InitNameClassTable
  (bind _nameclasstable (Variables|Default|GetNameClassTable))
  (bind _nameclasstable_2 (Variables|Default|GetNameClassTable))
  (Utilities|FlowControl|Sequence
    (:then_0
      ;[0.66 0.2868 0] Wood
      (Utilities|Array|Add _nameclasstable_2 (Utilities|Struct|MakeNameClassItem "Wood_C" "/Game/BluePrintAntonin/Items/Wood.Wood_C")))
    (:then_1
      ;[0.275 0.1551 0.07675] Stone
      (Utilities|Array|Add _nameclasstable_2 (Utilities|Struct|MakeNameClassItem "Stone_C" "/Game/BluePrintAntonin/Items/Stone.Stone_C")))
    (:then_2
      ;[1 0.5087 0.4896] Little_House_Wood
      (Utilities|Array|Add _nameclasstable_2 (Utilities|Struct|MakeNameClassItem "Little_House_Wood" "/Game/BluePrintAntonin/Items/Little_House_Wood.Little_House_Wood_C")))
    (:then_3
      ;[0.095 0.045 0.01329] Weapon_Axe
      (Utilities|Array|Add _nameclasstable_2 (Utilities|Struct|MakeNameClassItem "Weapon_Axe" "/Game/BluePrintAntonin/Weapon/Weapon_Axe.Weapon_Axe_C")))
    (:then_4
      ;[0.1732 1 0.1412] Apple
      (Utilities|Array|Add _nameclasstable_2 (Utilities|Struct|MakeNameClassItem "Apple_C" "/Game/BluePrintAntonin/Items/Apple.Apple_C")))
    (:then_5
      ;[0.47 0.1132 0] Planche de bois
      (Utilities|Array|Add _nameclasstable_2 (Utilities|Struct|MakeNameClassItem "Wood_Planche" "/Game/BluePrintAntonin/Items/Wood_Planche.Wood_Planche_C")))
    (:then_6
      ;[1 1 1] Weapon_Sword
      (Utilities|Array|Add _nameclasstable_2 (Utilities|Struct|MakeNameClassItem "Weapon_Sword" "/Game/BluePrintAntonin/Weapon/Weapon_Sword.Weapon_Sword_C")))
    (:then_7
      (Utilities|FlowControl|Sequence
        (:then_0
          ;[1 1 1] Metal
          (Utilities|Array|Add _nameclasstable (Utilities|Struct|MakeNameClassItem "Metal_C" "/Game/BluePrintAntonin/Items/Metal.Metal_C")))
        (:then_1
          ;[0.1574 0.565 0.1429] Green Crystal
          (Utilities|Array|Add _nameclasstable (Utilities|Struct|MakeNameClassItem "GreenCrystal_C" "/Game/BluePrintAntonin/Items/GreenCrystal.GreenCrystal_C")))
        (:then_2
          ;[1 1 1] !!!!!???
          (Utilities|Array|Add _nameclasstable (Utilities|Struct|MakeNameClassItem "LightSaberGreen" "/Game/BluePrintAntonin/Weapon/LightSaberGreen.LightSaberGreen_C")))
        (:then_3
          (Utilities|Array|Add _nameclasstable (Utilities|Struct|MakeNameClassItem "LightSaberRed" "/Game/BluePrintAntonin/Weapon/LightSaberRed.LightSaberRed_C")))
        (:then_4
          ;[1 0.1894 0.2181] Red Crystal
          (Utilities|Array|Add _nameclasstable (Utilities|Struct|MakeNameClassItem "RedCrystal_C" "/Game/BluePrintAntonin/Items/RedCrystal.RedCrystal_C")))
        (:then_5
          ;[0.4166 0.3222 1] PickAxe
          (Utilities|Array|Add _nameclasstable (Utilities|Struct|MakeNameClassItem "Weapon_PickAxe" "/Game/BluePrintAntonin/Weapon/Weapon_PickAxe.Weapon_PickAxe_C")))
        (:then_6
          ;[1 1 1] Machette
          (Utilities|Array|Add _nameclasstable (Utilities|Struct|MakeNameClassItem "Weapon_Machette" "/Game/BluePrintAntonin/Weapon/Weapon_Machette.Weapon_Machette_C")))))))

(fn SpawnInventorywithName
  (params (Invent :type Array%20of%20Strings))
  (for _array_element Invent
    (CallFunction|GetClasswithName _array_element)
    (bind _returnvalue (Game|SpawnActorfromClass (Variables|Default|GetClassFind) (Math|Transform|MakeTransform "10000.000000,10000.000000, 0") false 0))
    (bind _asbase_inventory_actor (Utilities|Casting|CastToBaseInventoryActor _returnvalue))
    (Variables|/Game/BluePrintAntonin/InventoryBP/BP_Inventory/BaseInventoryActor.BaseInventoryActor_C|SetInventoryClass _asbase_inventory_actor "/Game/BluePrintAntonin/InventoryBP/BP_Inventory/BP_CHILD_InventoryMain.BP_CHILD_InventoryMain_C")
    (Utilities|Array|Add (Variables|Default|GetTempInventory) _asbase_inventory_actor))
  (return (Variables|Default|GetTempInventory)))

(fn SpawnMyPlayer
  (params (Name :type Name) (Player :type Character%20Anto%20Object%20Reference))
  (bind _savegameinstance (Variables|Saveandload|GetSaveGameInstance))
  (Saveandload|LoadGame)
  (bind _index (Default|GetIndexOfPlayerwithName _savegameinstance Name))
  (bind _inventory (CallFunction|SpawnInventoryWithname (.InventoryString (Utilities|Struct|BreakSaveStructData (Utilities|Array|Get(acopy) (Variables|/Game/Blueprints/SavingGame/SaveData.SaveData_C|GetPlayers _savegameinstance) _index)))))
  (bind _arme (Outils|SpawnWeaponWithname (.WeaponString (Utilities|Struct|BreakSaveStructData (Utilities|Array|Get(acopy) (Variables|/Game/Blueprints/SavingGame/SaveData.SaveData_C|GetPlayers _savegameinstance) _index)))))
  (Default|InitMewithParameters Player _inventory (.CurrentInventoryAmount (Utilities|Struct|BreakSaveStructData (Utilities|Array|Get(acopy) (Variables|/Game/Blueprints/SavingGame/SaveData.SaveData_C|GetPlayers _savegameinstance) _index))) (.PreviousWorldPosition (Utilities|Struct|BreakSaveStructData (Utilities|Array|Get(acopy) (Variables|/Game/Blueprints/SavingGame/SaveData.SaveData_C|GetPlayers _savegameinstance) _index))) _arme Name (.InfoTextDisplay (Utilities|Struct|BreakSaveStructData (Utilities|Array|Get(acopy) (Variables|/Game/Blueprints/SavingGame/SaveData.SaveData_C|GetPlayers _savegameinstance) _index))) (.Health (Utilities|Struct|BreakSaveStructData (Utilities|Array|Get(acopy) (Variables|/Game/Blueprints/SavingGame/SaveData.SaveData_C|GetPlayers _savegameinstance) _index)))))

(fn LoadGame
  (Utilities|FlowControl|Sequence
    (:then_0
      (bind _returnvalue (SaveGame|DoesSaveGameExist "Between_Menu_Save"))
      (if _returnvalue
        (bind _returnvalue_2 (SaveGame|LoadGamefromSlot "Between_Menu_Save"))
        (bind _assave_between_menu (Utilities|Casting|CastToSaveBetweenMenu _returnvalue_2))
        (Variables|Saveandload|SetNamePlayerToSpawn (Variables|/Game/Blueprints/SavingGame/SaveBetweenMenu.SaveBetweenMenu_C|GetNamePlayer _assave_between_menu))
        (Variables|Saveandload|SetIsNewplayer (Variables|/Game/Blueprints/SavingGame/SaveBetweenMenu.SaveBetweenMenu_C|GetIsNewCharacter _assave_between_menu))))
    (:then_1
      (bind _returnvalue_3 (SaveGame|DoesSaveGameExist "SauvegardeRebornSociety"))
      (if _returnvalue_3
        (Variables|Saveandload|SetSaveExist true)
        (bind _returnvalue_4 (SaveGame|LoadGamefromSlot "SauvegardeRebornSociety"))
        (bind _assave_data (Utilities|Casting|CastToSaveData _returnvalue_4))
        (Variables|Saveandload|SetSaveGameInstance _assave_data)
        (Saveandload|LoadDatafromSaveFile)
        (else
          (Variables|Saveandload|SetSaveExist false))))))

(fn LoadDatafromSaveFile
  (bind _savegameinstance (Variables|Saveandload|GetSaveGameInstance))
  (bind _players (Variables|/Game/Blueprints/SavingGame/SaveData.SaveData_C|GetPlayers _savegameinstance))
  (Variables|Saveandload|SetPreviousSavePlayers _players)
  (for _array_element _players
    (Utilities|Array|Add (Variables|Saveandload|GetPlayersExist) (.Name (Utilities|Struct|BreakSaveStructData _array_element)))))

(fn CheckifPlayerExist
  (params (name :type Name))
  (for _array_element (Variables|Saveandload|GetPlayersExist)
    (if (Utilities|Name|Equal(Name) _array_element name)
      (return (Utilities|Name|Equal(Name) _array_element name)))))

(fn InitDataCraft
  (bind _datacraft (Variables|Default|GetDataCraft))
  ;[1 1 1] Little house wood
  (Utilities|Array|Add _datacraft (Utilities|Struct|MakeRowStruct "Little_House_Wood" "Wood_Planche_C" "Wood_Planche_C"))
  ;[1 1 1] Axe
  (Utilities|Array|Add _datacraft (Utilities|Struct|MakeRowStruct "Weapon_Axe" "Wood_C" "Stone_C"))
  ;[1 1 1] Planche
  (Utilities|Array|Add _datacraft (Utilities|Struct|MakeRowStruct "Wood_Planche" "Wood_C" "Wood_C"))
  ;[1 1 1] Sword
  (Utilities|Array|Add _datacraft (Utilities|Struct|MakeRowStruct "Weapon_Sword" "Metal_C" "Metal_C"))
  ;[1 1 1] !!!!!!?????
  (Utilities|Array|Add _datacraft (Utilities|Struct|MakeRowStruct "LightSaberGreen" "Metal_C" "GreenCrystal_C"))
  (Utilities|Array|Add _datacraft (Utilities|Struct|MakeRowStruct "LightSaberRed" "Metal_C" "RedCrystal_C"))
  ;[1 1 1] PickAxe
  (Utilities|Array|Add _datacraft (Utilities|Struct|MakeRowStruct "Weapon_PickAxe" "Wood_C" "Metal_C"))
  ;[1 1 1] Machette
  (Utilities|Array|Add _datacraft (Utilities|Struct|MakeRowStruct "Weapon_Machette" "Stone_C" "Stone_C")))